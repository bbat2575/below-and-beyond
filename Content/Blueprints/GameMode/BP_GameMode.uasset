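; Game mode that tracks crystal pickup progress for a level.
; On BeginPlay it records the number of BP_Crystal actors as the total and creates and stores a center message widget, without adding it to the viewport here.
; CrystalCountText recounts live crystals on each call and returns text labelled "Crystals Remaining", though the first number is the count already gone, shown against the total.
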(event EventBeginPlay
  (bind _outactors (Actor|GetAllActorsOfClass "/Game/Blueprints/Actors/Collectibles/BP_Crystal.BP_Crystal_C"))
  (Variables|Default|SetTotalCrystals (Utilities|Array|Length _outactors))
  (bind _returnvalue (UserInterface|CreateWidget "/Game/Blueprints/UI/WBP_CenterMessage.WBP_CenterMessage_C"))
  (Variables|Default|SetWBPCenterMessage _returnvalue))

(event EventTick
  (params (DeltaSeconds :type Float%20%28single-precision%29)))

(fn ConstructionScript)

(fn CrystalCountText
  (bind _totalcrystals (Variables|Default|GetTotalCrystals))
  (bind _outactors (Actor|GetAllActorsOfClass "/Game/Blueprints/Actors/Collectibles/BP_Crystal.BP_Crystal_C"))
  (return (Utilities|Text|ToText(String) (Utilities|String|Append "Crystals Remaining: " (Utilities|String|ToString(Integer) (- _totalcrystals (Utilities|Array|Length _outactors))) "/" (Utilities|String|ToString(Integer) _totalcrystals)))))