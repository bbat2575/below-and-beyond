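; Player ball pawn that rolls by applying input-driven torque to its physics mesh and restarts the level with a camera fade on any damage.
; Tick uses a sphere trace for ground contact and velocity for speed-scaled rolling audio, enabled after the opening fade.
; Hit plays wall bumps from the surface normal, plus landing bounces through a DoOnce re-armed while airborne.
; AdjustSpringArm lets Level 2 change camera distance and pitch.
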(event EventBeginPlay
  ;[0.1354 0.1628 1] Adjust Camera + Audio Activation
  (CameraFades|StartCameraFade :self (Game|GetPlayerCameraManager 0) :FromAlpha 1.0 :Duration 1.0)
  (Utilities|FlowControl|Delay 1.0)
  (Variables|Default|SetAudioOn true))

(event Collision|EventActorBeginOverlap
  (params (OtherActor :type Actor%20Object%20Reference))
  ;[0.1354 0.1628 1] Adjust Camera + Audio Activation
)

(event EventTick
  (params (DeltaSeconds :type Float%20%28single-precision%29))
  (bind _returnvalue (Transformation|GetActorLocation))
  (bind _ballbounce (Variables|Default|GetBallBounce))
  (bind _returnvalue_2 (+ (.z _returnvalue) -5e+01))
  ;[0.1667 1 0.3586] Rolling Sound + Ground/Surface Contact Detection
  ;;[1 1 1] Adjust rolling volume with speed
  (Audio|Components|Audio|SetVolumeMultiplier (Variables|Default|GetRollingAudio) (/ (Variables|Default|GetCurrentSpeed) 1.5e+03) :!class /Script/Engine.AudioComponent)
  ;;[1 1 1] Check if there's contact with any surface/ground
  (bind _returnvalue_3 (Collision|MultiSphereTraceByChannel (Math|Vector|MakeVector (.x _returnvalue) (.y _returnvalue) _returnvalue_2) (Math|Vector|MakeVector (.x _returnvalue) (.y _returnvalue) _returnvalue_2) 55.0 "TraceTypeQuery1" false 0 "None"))
  (bind _output_get (Variables|Default|SetIsGrounded _returnvalue_3))
  (Utilities|FlowControl|Sequence
    (:then_0
      (if (and (not _output_get) (not _returnvalue_3))
        ;[1 0.9186 0.1667] Play Ball Bumping + Bouncing Sounds
        ;;[1 1 1] Bounding Off The Floor Sound
        (Utilities|FlowControl|DoOnce false) ; enters at Reset
      ))
    (:then_1
      (bind _returnvalue_4 (Physics|GetPhysicsLinearVelocity (Variables|Default|GetMesh) "None"))
      (Variables|Default|SetCurrentSpeed (Math|Vector|VectorLength _returnvalue_4))
      (Utilities|FlowControl|Sequence
        (:then_0
          (if (Math|Boolean|ANDBoolean (Variables|Default|GetIsGrounded) (> (Variables|Default|GetCurrentSpeed) 1e+01) (Variables|Default|GetAudioOn))
            (if (not (Audio|Components|Audio|IsPlaying (Variables|Default|GetRollingAudio)))
              (Audio|Components|Audio|Play (Variables|Default|GetRollingAudio) 0.0))
            (else
              (Audio|Components|Audio|Stop (Variables|Default|GetRollingAudio)))))))))

(event Game|Damage|EventAnyDamage
  (params (Damage :type Float%20%28single-precision%29) (DamageType :type Damage%20Type%20Object%20Reference) (InstigatedBy :type Controller%20Object%20Reference) (DamageCauser :type Actor%20Object%20Reference))
  ;[0.6891 0.1979 1] Movement
  (Utilities|RestartLevel))

(event Collision|EventHit
  (params (MyComp :type Primitive%20Component%20Object%20Reference) (Other :type Actor%20Object%20Reference) (OtherComp :type Primitive%20Component%20Object%20Reference) (bSelfMoved :type Boolean) (HitLocation :type Vector :default "0, 0, 0") (HitNormal :type Vector :default "0, 0, 0") (NormalImpulse :type Vector :default "0, 0, 0") (Hit :type Hit%20Result%20Structure%20%28by%20ref%29))
  (bind _ballbounce (Variables|Default|GetBallBounce))
  (bind _ballbump (Variables|Default|GetBallBump))
  ;[1 0.9186 0.1667] Play Ball Bumping + Bouncing Sounds
  (Utilities|FlowControl|Sequence
    (:then_0
      ;;[1 1 1] Bounding Off The Floor Sound
      (Utilities|FlowControl|DoOnce false
        (:Completed
          (if (and (not (Audio|Components|Audio|IsPlaying _ballbounce)) (not (Audio|Components|Audio|IsPlaying (Variables|Default|GetBallBump))))
            (Audio|Components|Audio|Play _ballbounce 0.0)))))
    (:then_1
      ;;[1 1 1] Bumping Into Walls Sound
      (if (< (.z (.Normal (Collision|BreakHitResult Hit))) 0.5)
        (if (and (not (Audio|Components|Audio|IsPlaying _ballbump)) (not (Audio|Components|Audio|IsPlaying (Variables|Default|GetBallBounce))))
          (Audio|Components|Audio|Play _ballbump 0.0))))))

(event Input|AxisEvents|InputAxisMoveForwards/Backwards
  (params (AxisValue :type Float%20%28single-precision%29))
  ;[0.6891 0.1979 1] Movement
  (Class|PrimitiveComponent|AddTorqueinRadians (Variables|Default|GetMesh) (Math|Vector|MakeVector 0.0 (* AxisValue (Variables|Default|Gettorque_strength)) 0.0) "None" true))

(event Input|AxisEvents|InputAxisMoveRight/Left
  (params (AxisValue :type Float%20%28single-precision%29))
  ;[0.6891 0.1979 1] Movement
  (Class|PrimitiveComponent|AddTorqueinRadians (Variables|Default|GetMesh) (Math|Vector|MakeVector (* AxisValue (Variables|Default|Gettorque_strength)) 0.0 0.0) "None" true))

(fn ConstructionScript)

(fn AdjustSpringArm
  (params (Distance :type Float%20%28double-precision%29) (Pitch :type Float%20%28double-precision%29))
  (bind _springarm (Variables|Default|GetSpringArm))
  ;[0.7677 0.2448 1] Only Level 2 calls this function to adjust camera angle + distance.
  (Variables|/Script/Engine.SpringArmComponent|SetTargetArmLength _springarm Distance)
  (Transformation|SetWorldRotation _springarm (Math|Rotator|MakeRotator 0.0 Pitch 0.0) false false))