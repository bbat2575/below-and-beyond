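; BP_Cannon is a cannon actor that automatically fires projectiles on a repeating cycle from BeginPlay.
; After a CannonFireRate delay, it spawns a scaled BP_Projectile at ProjectileSpawnPoint and plays an attenuated firing sound at an X-offset location.
; CannonFireTimeline then animates the barrel along local Y, and its Cannon Fired output loops back to the delay for the next shot.
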(event EventBeginPlay
  (bind _returnvalue (Transformation|GetActorLocation))
  (Utilities|FlowControl|Delay (Variables|CanonProperties|GetCannon%20Fire%20Rate) :!label _label)
  (CallFunction|SpawnProjectile)
  (Audio|PlaySoundatLocation "/Game/Audio/cannon_fire.cannon_fire" (Math|Vector|MakeVector (+ (Variables|Default|GetXOffset) (.x _returnvalue)) (.y _returnvalue) (.z _returnvalue)) "0.000000,0.000000,0.000000" 0.35 1.0 0.0 "/Game/Audio/ATT_Cannons.ATT_Cannons" 0 0 0)
  (bind _cannon_barrel_location (Timeline|Cannon%20Fire%20Timeline PlayFromStart)
    (:Update
      (CallFunction|MoveCannonBarrel _cannon_barrel_location))
    (:Cannon%20Fired
      (goto _label))))

(fn ConstructionScript)

(fn SpawnProjectile
  (bind _projectile_spawn_point (Variables|Default|GetProjectile%20Spawn%20Point))
  (Game|SpawnActorfromClass "/Game/Blueprints/Actors/Projectiles/BP_Projectile.BP_Projectile_C" (Math|Transform|MakeTransform (Transformation|GetWorldLocation _projectile_spawn_point) (Transformation|GetWorldRotation _projectile_spawn_point) (Math|Conversions|ToVector(Float) (Variables|CanonProperties|GetProjectile%20Scale))) "Undefined" "OverrideRootScale" 0 0))

(fn MoveCannonBarrel
  (params (Cannon%20Barrel%20Y%20Location :type Float%20%28double-precision%29))
  (Transformation|SetRelativeLocation (Variables|Default|GetCannon%20Barrel) (Math|Vector|MakeVector 0.0 Cannon%20Barrel%20Y%20Location 0.0) false false))