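; Level trigger that starts the giant alien encounter when the player pawn overlaps it, then disables its own collision.
; It spawns BP_GiantAlien at the referenced SpawnPoint actor and stores it on BP_GameMode.
; Two looping timers then keep spawning BP_AlienSkull at random offsets around that point, a faster one at its height and a slower one raised above it.
; Nothing here clears the timers.
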(event Custom|SpawnAlienSkulls
  (bind _spawnpoint (Variables|Default|GetSpawnPoint))
  (bind _returnvalue (Transformation|GetActorTransform _spawnpoint))
  (Game|SpawnActorfromClass "/Game/Blueprints/Actors/Projectiles/BP_AlienSkull.BP_AlienSkull_C" (Math|Transform|MakeTransform (+ (.location _returnvalue) (Math|Vector|MakeVector (Math|Random|RandomFloatinRange -1e+02 1e+02) (Math|Random|RandomFloatinRange -5e+02 5e+02) (Math|Random|RandomFloatinRange 0.0 0.0))) (.rotation _returnvalue) "1.000000,1.000000,1.000000") "Undefined" "MultiplyWithRoot" 0 0))

(event Custom|SpawnAlienSkulls2
  (Game|SpawnActorfromClass "/Game/Blueprints/Actors/Projectiles/BP_AlienSkull.BP_AlienSkull_C" (Math|Transform|MakeTransform (+ (.location (Transformation|GetActorTransform (Variables|Default|GetSpawnPoint))) (Math|Vector|MakeVector (Math|Random|RandomFloatinRange -1e+02 1e+02) (Math|Random|RandomFloatinRange -5e+02 5e+02) (Math|Random|RandomFloatinRange 2e+02 5e+02))) "0, 0, 0" "1.000000,1.000000,1.000000") "Undefined" "MultiplyWithRoot" 0 0))

(event EventBeginPlay)

(event Collision|EventActorBeginOverlap
  (params (OtherActor :type Actor%20Object%20Reference))
  (bind _spawnpoint (Variables|Default|GetSpawnPoint))
  (bind _returnvalue (Transformation|GetActorTransform _spawnpoint))
  (Utilities|Casting|CastToBP_PlayerPawn OtherActor)
  (bind _returnvalue_2 (Game|SpawnActorfromClass "/Game/Blueprints/Actors/GiantAlien/BP_GiantAlien.BP_GiantAlien_C" (Math|Transform|MakeTransform (.location _returnvalue) (.rotation _returnvalue) "1.000000,1.000000,1.000000") "Undefined" "MultiplyWithRoot" 0 0))
  (Collision|SetActorEnableCollision false)
  (bind _asbp_game_mode (Utilities|Casting|CastToBP_GameMode (Game|GetGameMode)))
  (Variables|/Game/Blueprints/GameMode/BP_GameMode.BP_GameMode_C|SetGiantAlien _asbp_game_mode _returnvalue_2)
  (Utilities|Time|SetTimerbyEvent (delegate Custom|SpawnAlienSkulls) 0.6 true)
  (Utilities|Time|SetTimerbyEvent (delegate Custom|SpawnAlienSkulls2) 1.2 true))

(event EventTick
  (params (DeltaSeconds :type Float%20%28single-precision%29)))

(fn ConstructionScript)