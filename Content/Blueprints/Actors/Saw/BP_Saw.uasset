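; BP_Saw is a moving saw blade hazard that damages actors it hits.
; On BeginPlay it copies MovementDistance into the InterpToMovement component's control points and finalises them, setting the path it travels.
; Tick spins the SawBlade component in yaw by BladeRotationSpeed each frame, without delta-time scaling, and the Hit event applies a fixed damage to the other actor.
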(event EventBeginPlay
  (CallFunction|SetInterptoMovementControlPoints))

(event Collision|EventActorBeginOverlap
  (params (OtherActor :type Actor%20Object%20Reference)))

(event EventTick
  (params (DeltaSeconds :type Float%20%28single-precision%29))
  (Transformation|AddLocalRotation (Variables|Default|Getsaw_blade) (Math|Rotator|MakeRotator 0.0 0.0 (Variables|Default|GetBlade%20Rotation%20Speed)) false false))

(event Collision|EventHit
  (params (MyComp :type Primitive%20Component%20Object%20Reference) (Other :type Actor%20Object%20Reference) (OtherComp :type Primitive%20Component%20Object%20Reference) (bSelfMoved :type Boolean) (HitLocation :type Vector :default "0, 0, 0") (HitNormal :type Vector :default "0, 0, 0") (NormalImpulse :type Vector :default "0, 0, 0") (Hit :type Hit%20Result%20Structure%20%28by%20ref%29))
  (Game|Damage|ApplyDamage Other 1.0 0 0))

(fn ConstructionScript)

(fn SetInterptoMovementControlPoints
  (Variables|/Script/Engine.InterpToMovementComponent|SetControlPoints (Variables|Default|GetInterpToMovement) (Variables|Default|GetMovement%20Distance))
  (Class|InterptoMovementComponent|FinaliseControlPoints (Variables|Default|GetInterpToMovement)))