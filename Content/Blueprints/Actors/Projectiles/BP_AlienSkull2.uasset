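; BP_AlienSkull2 is an alien skull actor that sways back and forth while rocking in pitch.
; On BeginPlay, IsSkull2 selects one of two movement events, run on a looping timer at about 60 Hz instead of Tick.
; Each adds sine-of-game-time deltas: MoveSkull along world X, MoveSkull2 along world Y with a Skull2Offset phase and reversed pitch.
; Overlap, Tick and the construction script are empty.
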(event Custom|Move%20Skull%202
  (Transformation|AddActorWorldOffset (Math|Vector|MakeVector 0.0 (* (Math|Trig|Sin(Degrees) (* (+ (Utilities|Time|GetGameTimeinSeconds) (Variables|Default|GetSkull2Offset)) 1e+02)) 5.0) 0.0))
  (Transformation|AddActorLocalRotation (Math|Rotator|MakeRotator 0.0 (* (Math|Trig|Sin(Degrees) (* (+ (Utilities|Time|GetGameTimeinSeconds) -1e+02) 1e+02)) 0.8) 0.0) false false))

(event Custom|Move%20Skull
  (Transformation|AddActorWorldOffset (Math|Vector|MakeVector (* (Math|Trig|Sin(Degrees) (* (+ (Utilities|Time|GetGameTimeinSeconds) -100.66668) 1e+02)) 5.0) 0.0 0.0))
  (Transformation|AddActorLocalRotation (Math|Rotator|MakeRotator 0.0 (* (Math|Trig|Sin(Degrees) (* (+ (Utilities|Time|GetGameTimeinSeconds) -1e+02) -1e+02)) 0.8) 0.0) false false))

(event EventBeginPlay
  (if (Variables|Default|GetIsSkull2)
    (Utilities|Time|SetTimerbyEvent (delegate Custom|Move%20Skull%202) 0.016667 true)
    (else
      (Utilities|Time|SetTimerbyEvent (delegate Custom|Move%20Skull) 0.016667 true))))

(event Collision|EventActorBeginOverlap
  (params (OtherActor :type Actor%20Object%20Reference)))

(event EventTick
  (params (DeltaSeconds :type Float%20%28single-precision%29)))

(fn ConstructionScript)