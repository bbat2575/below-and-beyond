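; BP_WinVolume is the level exit volume, which lets the player finish once every crystal is gone.
; On player overlap, any remaining BP_Crystal actors trigger a center message with the count, taken from the game mode's widget, which fades out after a delay.
; Otherwise it finds the current map in LevelNames, then shows a loading screen and opens the next level, or shows the ending screen and quits on the last.
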(event Collision|EventActorBeginOverlap
  (params (OtherActor :type Actor%20Object%20Reference))
  (Utilities|IsPlayer OtherActor
    (:Is%20Player
      (if (CallFunction|AnyCrystalsRemaining)
        (bind _outactors (Actor|GetAllActorsOfClass "/Game/Blueprints/Actors/Collectibles/BP_Crystal.BP_Crystal_C"))
        (bind _asbp_game_mode (Utilities|Casting|CastToBP_GameMode (Game|GetGameMode)))
        (Variables|/Script/UMG.TextBlock|SetText (Variables|/Game/Blueprints/UI/WBP_CenterMessage.WBP_CenterMessage_C|GetCollectAllText (Variables|/Game/Blueprints/GameMode/BP_GameMode.BP_GameMode_C|GetWBPCenterMessage _asbp_game_mode)) (Utilities|Text|ToText(String) (Utilities|String|Append "Go Back - " (Utilities|String|ToString(Integer) (Utilities|Array|Length _outactors)) " Crystals Still Remaining!")))
        (Variables|/Script/UMG.Widget|SetRenderOpacity (Variables|/Game/Blueprints/UI/WBP_CenterMessage.WBP_CenterMessage_C|GetCollectAllText (Variables|/Game/Blueprints/GameMode/BP_GameMode.BP_GameMode_C|GetWBPCenterMessage _asbp_game_mode)) 1.0)
        (UserInterface|Viewport|AddtoViewport (Variables|/Game/Blueprints/GameMode/BP_GameMode.BP_GameMode_C|GetWBPCenterMessage _asbp_game_mode) 0)
        (Utilities|FlowControl|Delay 2.0)
        (UserInterface|Animation|PlayAnimation (Variables|/Game/Blueprints/GameMode/BP_GameMode.BP_GameMode_C|GetWBPCenterMessage _asbp_game_mode) (Variables|/Game/Blueprints/UI/WBP_CenterMessage.WBP_CenterMessage_C|GetFadeOut (Variables|/Game/Blueprints/GameMode/BP_GameMode.BP_GameMode_C|GetWBPCenterMessage _asbp_game_mode)) 0.0 1 "Forward" 1.0 false)
        (elif (LevelManagement|IsFinalLevel)
          (bind _returnvalue (UserInterface|CreateWidget "/Game/Blueprints/UI/WBP_EndingScreen.WBP_EndingScreen_C"))
          (UserInterface|Viewport|AddtoViewport _returnvalue 0)
          (Utilities|FlowControl|Delay 2.0)
          (Game|QuitGame 0 "Quit" false)
          (else
            (bind _returnvalue_2 (UserInterface|CreateWidget "/Game/Blueprints/UI/WBP_LoadingScreen.WBP_LoadingScreen_C"))
            (UserInterface|Viewport|AddtoViewport _returnvalue_2 0)
            (Utilities|FlowControl|Delay 2.0)
            (LevelManagement|LoadNextLevel)))))))

(fn ConstructionScript)

(fn AnyCrystalsRemaining
  (bind _outactors (Actor|GetAllActorsOfClass "/Game/Blueprints/Actors/Collectibles/BP_Crystal.BP_Crystal_C"))
  (return (> (Utilities|Array|Length _outactors) 0)))

(fn GetCurrentLevelIndex
  (bind _returnvalue (Game|GetCurrentLevelName true))
  (return (Utilities|Array|FindItem (Variables|Default|GetLevel%20Names) (Utilities|String|StringToName _returnvalue))))

(fn IsFinalLevel
  (return (== (Utilities|Array|LastIndex (Variables|Default|GetLevel%20Names)) (LevelManagement|GetCurrentLevelIndex))))

(fn LoadNextLevel
  (Game|OpenLevel(byName) (LevelManagement|GetNextLevelName)))

(fn GetNextLevelName
  (return (Utilities|Array|Get(acopy) (Variables|Default|GetLevel%20Names) (+ (LevelManagement|GetCurrentLevelIndex) 1))))