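; Giant alien actor that moves through the level in two timeline-driven motions with rolling animation.
; On BeginPlay a timeline drifts it along negative X and upward while rolling it by the timeline's progress.
; A StartMoving event plays alien audio and runs a second timeline that pushes it faster along negative X with a gentler opposite roll.
; Both timelines serve as update ticks, applying delta-time-scaled offsets without sweeping rather than interpolating between positions.
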(event Custom|StartMoving
  (bind _returnvalue (Utilities|Time|GetWorldDeltaSeconds))
  (Audio|Components|Audio|Play (Variables|Default|GetAlienAudio2) 0.0)
  (bind _progress_2 (Timeline|Timeline_0 Play)
    (:Update
      (Transformation|AddActorWorldOffset (Math|Vector|MakeVector (* (Math|Float|MakeLiteralFloat -4.0) 1e+02 _returnvalue) 0.0 0.0))
      (Transformation|AddActorLocalRotation (Math|Rotator|MakeRotator (* _progress_2 0.5 _returnvalue) 0.0 0.0) false false))))

(event EventBeginPlay
  (bind _returnvalue (Utilities|Time|GetWorldDeltaSeconds))
  (bind _progress (Timeline|Timeline Play)
    (:Update
      (Transformation|AddActorWorldOffset (* (Math|Vector|MakeVector -1.0 0.0 2.0) 75.0 _returnvalue))
      (Transformation|AddActorLocalRotation (Math|Rotator|MakeRotator (* _progress -1e+01 _returnvalue) 0.0 0.0) false false))))

(event Collision|EventActorBeginOverlap
  (params (OtherActor :type Actor%20Object%20Reference)))

(event EventTick
  (params (DeltaSeconds :type Float%20%28single-precision%29)))

(fn ConstructionScript)