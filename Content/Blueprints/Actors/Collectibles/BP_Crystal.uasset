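; BP_Crystal is a collectible crystal that the player picks up by overlapping it.
; The overlap stores its starting location, scale and light intensity, then a DoOnce gate plays a sound and starts CollectionTimeline.
; The timeline drives lerps that pull the crystal toward the player's current position while shrinking it and fading its light.
; On finish, it decrements the crystal count in BP_GameMode and destroys itself.
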(event Collision|EventActorBeginOverlap
  (params (OtherActor :type Actor%20Object%20Reference))
  (Utilities|IsPlayer OtherActor
    (:Is%20Player
      (CallFunction|StoreStartingValues)
      (Utilities|FlowControl|DoOnce false
        (:Completed
          (Audio|PlaySoundatLocation "/Game/Audio/crystal_collect.crystal_collect" (Transformation|GetActorLocation) "0, 0, 0" 0.4 1.5 0.0 0 0 0 0)
          (bind (_direction _collection_progress _scale_progress _light_intensity) (Timeline|Collection%20Timeline Play)
            (:Update
              (CallFunction|MovetoPlayer _collection_progress)
              (CallFunction|ScaleCrystal _scale_progress)
              (CallFunction|AdjustLight _light_intensity))
            (:Finished
              (bind _asbp_game_mode (Utilities|Casting|CastToBP_GameMode (Game|GetGameMode)))
              (Default|DecrementCrystalCount _asbp_game_mode)
              (Actor|DestroyActor))))))))

(fn ConstructionScript)

(fn MovetoPlayer
  (params (Alpha :type Float%20%28double-precision%29))
  (Transformation|SetActorLocation (Math|Vector|Lerp(Vector) (Variables|Default|GetStart%20Location) (Transformation|GetActorLocation (Game|Player|GetPlayerPawn 0)) Alpha) false false))

(fn StoreStartingValues
  (Variables|Default|SetStart%20Location (Transformation|GetActorLocation))
  (Variables|Default|SetStart%20Scale (Transformation|GetActorScale3D))
  (Variables|Default|SetStart%20Light%20Intensity (Variables|/Script/Engine.LightComponentBase|GetIntensity (Variables|Default|GetCrystal%20Light))))

(fn ScaleCrystal
  (params (Alpha :type Float%20%28double-precision%29))
  (Transformation|SetActorScale3D (Math|Vector|Lerp(Vector) (Variables|Default|GetStart%20Scale) "0, 0, 0" Alpha)))

(fn AdjustLight
  (params (Alpha :type Float%20%28double-precision%29))
  (Rendering|Components|Light|SetIntensity (Variables|Default|GetCrystal%20Light) (Math|Float|Lerp (Variables|Default|GetStart%20Light%20Intensity) 0.0 Alpha)))