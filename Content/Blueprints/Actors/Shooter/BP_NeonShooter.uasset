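; BP_NeonShooter is an actor that repeatedly fires BP_PathLights actors as projectiles.
; From BeginPlay it waits for the fire rate delay, spawns a projectile and plays CannonFireTimeline from the start.
; The timeline's Cannon Fired event loops back to the delay, so firing continues indefinitely.
; Projectiles take their location and rotation from ProjectileSpawnPoint and their scale from ProjectileScale.
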(event EventBeginPlay
  (Utilities|FlowControl|Delay (Variables|CanonProperties|GetCannon%20Fire%20Rate) :!label _label)
  (CallFunction|SpawnProjectile)
  (Timeline|Cannon%20Fire%20Timeline PlayFromStart
    (:Cannon%20Fired
      (goto _label))))

(fn ConstructionScript)

(fn SpawnProjectile
  (bind _projectile_spawn_point (Variables|Default|GetProjectile%20Spawn%20Point))
  (Game|SpawnActorfromClass "/Game/Blueprints/Actors/Projectiles/BP_PathLights.BP_PathLights_C" (Math|Transform|MakeTransform (Transformation|GetWorldLocation _projectile_spawn_point) (Transformation|GetWorldRotation _projectile_spawn_point) (Math|Conversions|ToVector(Float) (Variables|CanonProperties|GetProjectile%20Scale))) "Undefined" "OverrideRootScale" 0 0))